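; Game mode Blueprint that handles player controller tracking and session cleanup on logout, with respawning marked as done in code.
; Controller swaps append the new controller to AllPlayerControllers, though that event is also marked as done in code.
; Logout passes the exiting BP_PlayerController to BP_GameInstance to destroy its session.
; RespawnPlayer is empty; its old spawn-at-random-PlayerStart-and-possess logic remains disconnected and never runs.
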(event Custom|RespawnPlayer
  (params (Player%20Controller :type Player%20Controller%20Object%20Reference) (Character%20Class :type Character%20Class%20Reference))
  ;[1 1 1] Done in Code
)

(event EventOnSwapPlayerControllers
  (params (OldPC :type Player%20Controller%20Object%20Reference) (NewPC :type Player%20Controller%20Object%20Reference))
  ;[1 1 1] Done in Code
  ;;[1 1 1] Track connected player controllers
  (Utilities|Array|Add (Variables|GameInfo|GetAllPlayerControllers) NewPC))

(event EventOnLogout
  (params (ExitingController :type Controller%20Object%20Reference))
  ;[1 1 1] BP Only
  ;[1 1 1] Destroy session caller in Game Instance
  (bind _asbp_player_controller (Utilities|Casting|CastToBP_PlayerController ExitingController))
  (bind _asbp_game_instance (Utilities|Casting|CastToBP_GameInstance (Game|GetGameInstance)))
  (Default|DestroySessionCallerBP _asbp_game_instance _asbp_player_controller))

(fn ConstructionScript)